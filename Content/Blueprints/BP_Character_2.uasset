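; BP_Character_2 is a character that homes in on the first player character.
; Every Tick it rotates its capsule with FindLookAtRotation toward the player, then moves a fixed step along the capsule's forward vector.
; The move uses SetActorLocation without sweep, so it ignores blocking collision, and its speed depends on frame rate because delta time is unused.
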(event EventBeginPlay)

(event Collision|EventActorBeginOverlap
  (params (OtherActor :type Actor%20Object%20Reference)))

(event EventTick
  (params (DeltaSeconds :type Float%20%28single-precision%29))
  (Utilities|FlowControl|Sequence
    (:then_0
      (Transformation|SetWorldRotation (Variables|Collision|GetCapsuleComponent) (Math|Rotator|FindLookatRotation (Transformation|GetActorLocation) (Transformation|GetActorLocation (Game|GetPlayerCharacter 0))) false false))
    (:then_1
      (Transformation|SetActorLocation (+ (Transformation|GetActorLocation) (* (Math|Vector|GetForwardVector (Variables|Collision|GetCapsuleComponent)) 1e+01)) false false))))

(fn ConstructionScript)